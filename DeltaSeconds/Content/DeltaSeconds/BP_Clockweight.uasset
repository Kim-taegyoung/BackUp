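; BP_Clockweight is an actor that swings its static mesh back and forth, like a clock weight.
; Tick plays or reverses a Timeline each frame according to IsReverse, which flips whenever the Timeline finishes.
; Timeline updates set the mesh's relative pitch to the curve value scaled by MaxRot and offset by StartRot, with roll and yaw held at zero.
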(event EventTick
  (params (DeltaSeconds :type Float%20%28single-precision%29))
  (if (Variables|Default|GetIsReverse)
    (bind _value (Timeline|타임라인_0 Reverse)
      (:Update
        (Transformation|SetRelativeRotation (Variables|Default|GetStaticMesh) (Math|Rotator|MakeRotator 0.0 (+ (* _value (Variables|Default|GetMaxRot)) (Variables|Default|GetStartRot)) 0.0) false false))
      (:Finished
        (Variables|Default|SetIsReverse (not (Variables|Default|GetIsReverse)))))
    (else
      (Timeline|타임라인_0 Play))))

(fn ConstructionScript)