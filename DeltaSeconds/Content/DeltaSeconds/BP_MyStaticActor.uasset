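; BP_MyStaticActor is an actor that rotates itself using values held on player controllers.
; Each Tick it loops over actors tagged "obj", using only the loop index to fetch a BP_MyPlayerController.
; That controller's X, Y and Z become the world rotation delta, unscaled by delta time.
; PrintRecivedEvent only prints a debug message and is not called within this Blueprint.
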(event EventTick
  (params (DeltaSeconds :type Float%20%28single-precision%29))
  (bind _outactors (Actor|GetAllActorswithTag "obj"))
  (for (_ _array_index) _outactors
    (bind _asbp_my_player_controller (Utilities|Casting|CastToBP_MyPlayerController (Game|GetPlayerController _array_index)))
    (Class|Actor|AddActorWorldRotation (Math|Rotator|MakeRotator (Variables|/Game/DeltaSeconds/BP_MyPlayerController.BP_MyPlayerController_C|GetX _asbp_my_player_controller) (Variables|/Game/DeltaSeconds/BP_MyPlayerController.BP_MyPlayerController_C|GetY _asbp_my_player_controller) (Variables|/Game/DeltaSeconds/BP_MyPlayerController.BP_MyPlayerController_C|GetZ _asbp_my_player_controller)))))

(fn ConstructionScript)

(fn PrintRecivedEvent
  (Development|PrintString "Recived Event"))