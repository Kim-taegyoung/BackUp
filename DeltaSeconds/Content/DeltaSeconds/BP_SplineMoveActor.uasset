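; Actor that moves a cube back and forth along its spline, rotating it to follow the curve.
; Each Tick places the cube at the transform for the current distance along the spline, keeping its own scale.
; A direction flag steps that distance up or down by one unit per frame, flipping at either end of the spline.
; Movement is frame-rate dependent, since delta time is not used.
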(event EventTick
  (params (DeltaSeconds :type Float%20%28single-precision%29))
  (bind _spline (Variables|Default|GetSpline))
  (bind _curdistance (Variables|Default|GetCurDistance))
  (bind _returnvalue (Spline|GetTransformatDistanceAlongSpline _spline _curdistance "World" false))
  ;[1 1 1] 스플라인 따라 움직이기
  ;;[1 1 1] 따라서 회전도 하는 큐브
  (Transformation|SetWorldTransform (Variables|Default|GetCube) (Math|Transform|MakeTransform (.location _returnvalue) (.rotation _returnvalue) (Transformation|GetWorldScale (Variables|Default|GetCube))) false false)
  (if (Variables|Default|GetIsMoveForward)
    ;;[1 1 1] MoveForward
    (bind _result (Math|Float|IncrementFloat (Variables|Default|GetCurDistance))
      (:%20%20
        (if (> _result (Spline|GetSplineLength (Variables|Default|GetSpline)))
          (Variables|Default|SetIsMoveForward false))))
    (else
      ;;[1 1 1] BackWard
      (bind _result_2 (Math|Float|DecrementFloat (Variables|Default|GetCurDistance))
        (:%20%20
          (if (< _result_2 0.0)
            (Variables|Default|SetIsMoveForward true)))))))

(fn ConstructionScript)