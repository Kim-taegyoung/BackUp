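; Door trap that continuously swings its static mesh open and closed.
; Tick checks IsOpen to run either UpdateOpen or UpdateClose, which rotate the mesh on local roll using separate open and close speeds.
; Each flips IsOpen when relative roll reaches its limit of 90 or zero degrees, looping the motion.
; Scaling rotation by DeltaSeconds keeps the speed frame-rate independent.
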(event EventTick
  (params (DeltaSeconds :type Float%20%28single-precision%29))
  (if (Variables|Default|GetIsOpen)
    (CallFunction|UpdateClose DeltaSeconds)
    (else
      (CallFunction|UpdateOpen DeltaSeconds))))

(fn ConstructionScript)

(fn UpdateOpen
  (params (DeltaSeconds :type Float%20%28single-precision%29))
  (bind _staticmesh (Variables|Default|GetStaticMesh))
  (Transformation|AddLocalRotation _staticmesh (Math|Rotator|MakeRotator (* DeltaSeconds (Variables|Default|GetOpenSpeed)) 0.0 0.0) false false)
  (if (>= (.roll (Variables|/Script/Engine.SceneComponent|GetRelativeRotation _staticmesh)) 9e+01)
    (Variables|Default|SetIsOpen true)))

(fn UpdateClose
  (params (DeltaSeconds :type Float%20%28single-precision%29))
  (bind _staticmesh (Variables|Default|GetStaticMesh))
  (bind _result (Math|Float|NegateFloat (* DeltaSeconds (Variables|Default|GetCloseSpeed)))
    (:%20%20
      (Transformation|AddLocalRotation _staticmesh (Math|Rotator|MakeRotator _result 0.0 0.0) false false)
      (if (<= (.roll (Variables|/Script/Engine.SceneComponent|GetRelativeRotation _staticmesh)) 0.0)
        (Variables|Default|SetIsOpen false)))))