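; BP_DeltaSeconds is a timer test Blueprint that builds clock strings from accumulated Tick delta time and prints them on screen.
; Tick feeds doubled delta time into CountSS, printing a wrapping seconds count with a Korean suffix only when the string changes.
; Unused alternatives provide a plain seconds counter, a countdown and an AM/PM hour-minute-second clock, the latter using zero-padding and AM/PM helpers.
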(event EventTick
  (params (DeltaSeconds :type Float%20%28single-precision%29))
  (bind _ss (CallFunction|CountSS (* 2 DeltaSeconds)))
  (if (not (Utilities|Enum|Equal(Enum) _ss (Variables|Default|GetBeforeStr)))
    (Variables|Default|SetBeforeStr _ss)
    (Development|PrintString _ss true true "(R=0.000000,G=0.660000,B=1.000000,A=1.000000)" 1e+02)))

(fn ConstructionScript)

(fn DeltaSecondsCounting
  (params (DeltaSeconds :type Float%20%28single-precision%29))
  ;[1 1 1] 59까지 반복
  (bind _output_get (Variables|Default|SetTotalDeltaSeconds (+ DeltaSeconds (Variables|Default|GetTotalDeltaSeconds))))
  (return (Utilities|String|ToString(Integer) (Math|Float|Floor (Math|Float|%(Float) _output_get 6e+01)))))

(fn CountTimeHHMMSS
  (params (DeltaSeconds :type Float%20%28single-precision%29))
  (bind _output_get (Variables|Default|SetTotalDeltaSeconds (+ DeltaSeconds (Variables|Default|GetTotalDeltaSeconds))))
  (return (Utilities|String|Append (CallFunction|InttoAMPM (Math|Float|Floor (Math|Float|%(Float) (/ _output_get 4.32e+04) 2.0))) (CallFunction|InttoStr00 (Math|Float|Floor (Math|Float|%(Float) (/ _output_get 3.6e+03) 12.0))) "시" (CallFunction|InttoStr00 (Math|Float|Floor (Math|Float|%(Float) (/ _output_get 6e+01) 6e+01))) "분" (CallFunction|InttoStr00 (Math|Float|Floor (Math|Float|%(Float) _output_get 6e+01))) "초")))

(fn InttoStr00
  (params (Int :type Integer))
  ;[1 1 1] 한자릿 정수 앞에 0입력하기
  (if (< (Math|Conversions|ToByte(Integer) Int) 10)
    (return (Utilities|String|Append "0" (Utilities|String|ToString(Integer) Int)))
    (else
      (return (Utilities|String|ToString(Integer) Int)))))

(fn CountDown
  (params (DeltaSeconds :type Float%20%28single-precision%29))
  (bind _output_get (Variables|Default|SetCountingDown (- (Variables|Default|GetCountingDown) DeltaSeconds)))
  (return (Utilities|String|ToString(Integer) (Math|Float|Floor _output_get))))

(fn CountSS
  (params (DeltsSeconds :type Float%20%28single-precision%29))
  (bind _output_get (Variables|Default|SetTotalDeltaSeconds (+ DeltsSeconds (Variables|Default|GetTotalDeltaSeconds))))
  (return (Utilities|String|Append (Utilities|String|ToString(Integer) (Math|Float|Floor (Math|Float|%(Float) _output_get 6e+01))) "초")))

(fn InttoAMPM
  (params (Int :type Integer))
  (if (== Int 0)
    (return "AM")
    (else
      (return "PM"))))