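; Actor that shuttles a Cube back and forth along its Spline.
; Each Tick places the cube at the spline's location and rotation at the current distance, keeping its scale, then steps that distance, reversing at either end.
; A local rotation follows but does not accumulate, as the next tick resets rotation to the spline's.
; Steps are fixed per frame without delta time, so speed depends on frame rate.
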(event EventTick
  (params (DeltaSeconds :type Float%20%28single-precision%29))
  (Utilities|FlowControl|Sequence
    (:then_0
      (Transformation|SetWorldTransform (Variables|Default|GetCube) (Math|Transform|MakeTransform (.location (Spline|GetTransformatDistanceAlongSpline (Variables|Default|GetSpline) (Variables|Default|GetCurDistance) "World" false)) (.rotation (Spline|GetTransformatDistanceAlongSpline (Variables|Default|GetSpline) (Variables|Default|GetCurDistance) "World" false)) (Transformation|GetWorldScale (Variables|Default|GetCube))) false false)
      (if (Variables|Default|GetIsMoveForward)
        (Variables|Default|SetCurDistance (+ (Variables|Default|GetCurDistance) 1e+01))
        (if (> (Variables|Default|GetCurDistance) (Spline|GetSplineLength (Variables|Default|GetSpline)))
          (Variables|Default|SetIsMoveForward false))
        (else
          (Variables|Default|SetCurDistance (- (Variables|Default|GetCurDistance) 1e+01))
          (if (<= (Variables|Default|GetCurDistance) 0.0)
            (Variables|Default|SetIsMoveForward true)))))
    (:then_1
      (Transformation|AddLocalRotation (Variables|Default|GetCube) "0.000000,0.000000,10.000000" false false))))

(fn ConstructionScript)